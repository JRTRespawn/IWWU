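; BridgeTrigger is a trigger actor in Level00 that lets the player register an interaction while inside its box.
; On BeginPlay it creates an InteractTutorial widget, which box overlaps by the player character show or hide while enabling or disabling the actor's input.
; Pressing Interact sets the IsInteacted flag, with no further response in this Blueprint.
; A separate RemoveWidget event takes the prompt off screen.
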(event OnComponentBeginOverlap(Box)
  (params (OverlappedComponent :type Primitive%20Component%20Object%20Reference) (OtherActor :type Actor%20Object%20Reference) (OtherComp :type Primitive%20Component%20Object%20Reference) (OtherBodyIndex :type Integer) (bFromSweep :type Boolean) (SweepResult :type Hit%20Result%20Structure%20%28by%20ref%29))
  (if (and (== OtherActor (Game|GetPlayerCharacter 0)) (not (UserInterface|Viewport|IsinViewport (Variables|Default|GetWidgetInteract))))
    (UserInterface|Viewport|AddtoViewport (Variables|Default|GetWidgetInteract) 0)
    (Input|EnableInput (Game|GetPlayerController 0))))

(event OnComponentEndOverlap(Box)
  (params (OverlappedComponent :type Primitive%20Component%20Object%20Reference) (OtherActor :type Actor%20Object%20Reference) (OtherComp :type Primitive%20Component%20Object%20Reference) (OtherBodyIndex :type Integer))
  (if (and (== OtherActor (Game|GetPlayerCharacter 0)) (UserInterface|Viewport|IsinViewport (Variables|Default|GetWidgetInteract)))
    (Widget|RemovefromParent (Variables|Default|GetWidgetInteract))
    (Input|DisableInput (Game|GetPlayerController 0))))

(event Custom|RemoveWidget
  (bind _widgetinteract (Variables|Default|GetWidgetInteract))
  (if (UserInterface|Viewport|IsinViewport _widgetinteract)
    (Widget|RemovefromParent _widgetinteract)))

(event EventBeginPlay
  (bind _returnvalue (UserInterface|CreateWidget "/Game/IWAContent/UserInterface/Tutorial/InteractTutorial.InteractTutorial_C"))
  (Variables|Default|SetWidgetInteract _returnvalue))

(event Collision|EventActorBeginOverlap
  (params (OtherActor :type Actor%20Object%20Reference)))

(event EventTick
  (params (DeltaSeconds :type Float%20%28single-precision%29)))

(event Input|ActionEvents|InputActionInteract
  (params (Key :type Key%20Structure))
  (:Pressed
    (Variables|Default|SetisInteacted true)))

(fn ConstructionScript)