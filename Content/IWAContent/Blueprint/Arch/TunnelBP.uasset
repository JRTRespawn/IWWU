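; TunnelBP is a construction-script Blueprint that builds a tunnel as a straight row of repeated child actors.
; It adds TunnelNumber child actor components, spacing them at a fixed 147-unit interval along relative X from the first.
; Each piece takes its world scale from the scene root.
; An unconnected calculation that derives a count from the distance between Length and Root components is left unused.
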(fn ConstructionScript
  (for _index (range 1 (Variables|Default|GetTunnelNumber))
    (bind _returnvalue (AddComponent|AddChildActorComponent false (Transformation|GetActorTransform)))
    (Transformation|SetWorldScale3D _returnvalue (Transformation|GetWorldScale (Variables|Default|GetDefaultSceneRoot)))
    (Transformation|SetRelativeLocation _returnvalue (Math|Vector|MakeVector (* (- _index 1) 147.0) 0.0 0.0) false false)))