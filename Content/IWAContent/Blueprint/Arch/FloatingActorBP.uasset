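; FloatingActorBP is an actor that makes a configurable static mesh bob smoothly back and forth.
; The construction script adds the mesh component, applies the shadow setting and optionally overrides the first material slot.
; Each tick moves the actor by the change in a sine of accumulated running time, scaled per axis by X, Y and Z.
; Movement is relative to the current location, without sweep.
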(event EventTick
  (params (DeltaSeconds :type Float%20%28single-precision%29))
  (bind _returnvalue (Transformation|GetActorLocation))
  (Transformation|SetActorLocation (Math|Vector|MakeVector (+ (* (- (Math|Trig|Sin(Radians) (+ DeltaSeconds (Variables|Default|GetRunningTime))) (Math|Trig|Sin(Radians) (Variables|Default|GetRunningTime))) (Variables|Floating|GetX)) (.x _returnvalue)) (+ (* (- (Math|Trig|Sin(Radians) (+ DeltaSeconds (Variables|Default|GetRunningTime))) (Math|Trig|Sin(Radians) (Variables|Default|GetRunningTime))) (Variables|Floating|GetY)) (.y _returnvalue)) (+ (* (- (Math|Trig|Sin(Radians) (+ DeltaSeconds (Variables|Default|GetRunningTime))) (Math|Trig|Sin(Radians) (Variables|Default|GetRunningTime))) (Variables|Floating|GetZ)) (.z _returnvalue))) false false)
  (Variables|Default|SetRunningTime (+ (Variables|Default|GetRunningTime) DeltaSeconds)))

(fn ConstructionScript
  (bind _material (Variables|Floating|GetMaterial))
  (bind _returnvalue (AddComponent|AddStaticMeshComponent false))
  (Components|StaticMesh|SetStaticMesh _returnvalue (Variables|Floating|GetStaticMesh))
  (Rendering|SetCastShadow _returnvalue (Variables|Floating|GetCastShadow))
  (Utilities|IsValid _material
    (:Is%20Valid
      (Rendering|Material|SetMaterial _returnvalue 0 _material))))